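; Space shooter enemy Blueprint that sets a diagonal MovementVector, extending its parent's BeginPlay and overlap logic.
; On BeginPlay it randomly picks one of two diagonals, both toward negative X with opposite Y.
; Overlapping an actor tagged "Lateral" multiplies the vector to invert Y and zero X and Z, leaving purely sideways movement.
; The file only sets the vector and contains no code that applies it.
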(event EventBeginPlay
  (|CallParentFunction)
  (if (Math|Random|RandomBool)
    (Variables|Default|SetMovementVector "-1.000000,-1.000000,0.000000")
    (else
      (Variables|Default|SetMovementVector "-1.000000,1.000000,0.000000"))))

(event Collision|EventActorBeginOverlap
  (params (OtherActor :type Actor%20Object%20Reference))
  (|CallParentFunction OtherActor)
  (if (Utilities|Array|ContainsItem (Variables|/Script/Engine.Actor|GetTags OtherActor) "Lateral")
    (Variables|Default|SetMovementVector (* (Variables|Default|GetMovementVector) "0.000000,-1.000000,0.000000"))))

(fn ConstructionScript
  (|CallParentFunction))