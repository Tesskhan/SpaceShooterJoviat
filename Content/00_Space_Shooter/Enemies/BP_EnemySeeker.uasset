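; BP_EnemySeeker is a space shooter enemy that keeps facing the player and fires at a regular interval.
; Each Tick snaps its rotation toward player character 0 with a look-at rotation, with no smoothing.
; A timer accumulates delta time and, once it passes DelayShoot, calls Fire and resets to zero.
; The graph contains no movement logic or Fire implementation, and construction only calls the parent script.
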(event EventTick
  (params (DeltaSeconds :type Float%20%28single-precision%29))
  ;[1 1 1] Comment
  (Transformation|SetActorRotation (Math|Rotator|FindLookatRotation (Transformation|GetActorLocation) (Transformation|GetActorLocation (Game|GetPlayerCharacter 0))))
  (Variables|Default|SetShootCurrentTime (+ (Variables|Default|GetShootCurrentTime) DeltaSeconds))
  (if (> (Variables|Default|GetShootCurrentTime) (Variables|Default|GetDelayShoot))
    (CallFunction|Fire)
    (Variables|Default|SetShootCurrentTime 0.0)))

(fn ConstructionScript
  (|CallParentFunction))